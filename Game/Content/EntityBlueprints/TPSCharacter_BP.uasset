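; TPSCharacter_BP is a character Blueprint that makes network authority handovers visible by changing its mesh material.
; Tick compares the current authority against a HadAuthority flag to detect changes, incrementing GainedAuthorityCount each time authority is gained.
; The count's RepNotify alternates mesh material slot 0 between the purple team material on odd counts and the red one on even counts.
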(event `self.ReceiveTick`
  (params (DeltaSeconds :type "Float (single-precision)"))
  (if (`self.HadAuthority`)
    (`/Engine/EditorBlueprintResources/ActorMacros.Switch Has Authority`
      (:`Remote`
        (set `self.HadAuthority` false)))
    (else
      (`/Engine/EditorBlueprintResources/ActorMacros.Switch Has Authority`
        (:`Authority`
          (set `self.HadAuthority` true)
          (`/Engine/EditorBlueprintResources/StandardMacros.IncrementInt` (`self.GainedAuthorityCount`)))))))

(fn `OnRep_GainedAuthorityCount`
  (bind _mesh (`self.Mesh`))
  (if (== (mod (`self.GainedAuthorityCount`) 2) 1)
    (`PrimitiveComponent.SetMaterial` _mesh 0 (`self.PurpleTeamMaterial`))
    (else
      (`PrimitiveComponent.SetMaterial` _mesh 0 (`self.RedTeamMaterial`)))))

(fn `UserConstructionScript`)